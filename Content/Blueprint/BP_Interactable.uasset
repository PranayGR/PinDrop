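; BP_Interactable is an interactable actor that makes noise when something collides with it.
; Collided stores the walk state, reports a noise event at its location and flags the collision on BP_FirstPersonGameMode once.
; If the game mode allows it, it also plays a sound scaled by the saved SFX level.
; GetSoundLevel maps the stored walk state to a sound level, and VisualEnable sets whether the actor is hidden.
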(event `self.ReceiveBeginPlay`
  (bind _asbp_first_person_game_mode (cast `/Game/FirstPerson/Blueprints/BP_FirstPersonGameMode` (`GameplayStatics.GetGameMode`)))
  (set `self.GameMode_Ref` _asbp_first_person_game_mode))

(event `/Game/Blueprint/Interface/BPI_Interactable.Collided`
  (params (Velocity :type "Float (double-precision)") (Walk_State :type "/Game/FirstPerson/Blueprints/E_Movement Enum" :default "NewEnumerator0"))
  (bind _returnvalue (`self.K2_GetActorLocation`))
  (set `self.Walk State` Walk_State)
  (`|ExecutionSequence`
    (:`then_0`
      (`AISense_Hearing.ReportNoiseEvent` _returnvalue 1.0 self)
      (`/Engine/EditorBlueprintResources/StandardMacros.DoOnce` false
        (:`Completed`
          (`/Game/FirstPerson/Blueprints/BP_FirstPersonGameMode.SetCollidedWithItem` (`self.GameMode_Ref`) true))))
    (:`then_1`
      (if (`/Game/FirstPerson/Blueprints/BP_FirstPersonGameMode.can box play sound` (`self.GameMode_Ref`))
        (`GameplayStatics.PlaySoundAtLocation` (`self.Sound`) _returnvalue (struct) (`/Game/FirstPerson/Blueprints/BP_SaveSlot.SFXLevel` (`/Game/FirstPerson/Blueprints/BP_GameInstance.SaveSlotRef` (cast `/Game/FirstPerson/Blueprints/BP_GameInstance` (`GameplayStatics.GetGameInstance`) :!pure true))) 1.0 0.0 null null null null)))))

(event `/Game/Blueprint/Interface/BPI_Interactable.VisualEnable`
  (params (Hidden :type Boolean))
  (`self.SetActorHiddenInGame` Hidden))

(fn `GetSoundLevel`
  (returns (SoundLevel :type "Float (double-precision)"))
  (return (select `/Game/FirstPerson/Blueprints/E_Movement` (`self.Walk State`) :`NewEnumerator0` (`self.Normal_Soundlevel`) :`NewEnumerator1` (`self.Sprint_Soundlevel_0`) :`NewEnumerator2` (`self.Crouch_Soundlevel`) :`NewEnumerator3` (`self.Slower Normal Walk SoundLevel`) :!type "Float (double-precision)")))

(fn `UserConstructionScript`)