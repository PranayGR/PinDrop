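; Level exit door that, on interaction, swings open when active or plays a locked sound and rotation animation otherwise.
; Opening triggers once the win screen, achievement check, completion flag and best-time save through the player controller and GameInstance.
; In parallel, timelines animate a point light and lerp the player to face the door, then into the room.
; PlayerInfo arrives via a controller event, with a delayed fallback read.
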(event `self.ReceiveBeginPlay`
  (bind _asbp_first_person_player_controller (cast `/Game/FirstPerson/Blueprints/BP_FirstPersonPlayerController` (`GameplayStatics.GetPlayerController` 0)))
  (add `/Game/FirstPerson/Blueprints/BP_FirstPersonPlayerController.PlayerInfoAdded` _asbp_first_person_player_controller (delegate `SetPlayerInfo`))
  (`KismetSystemLibrary.Delay` 3.0)
  (`/Engine/EditorBlueprintResources/StandardMacros.IsValid` (`self.PlayerInfoRef`)
    (:`Is Not Valid`
      (bind _asbp_first_person_player_controller_2 (cast `/Game/FirstPerson/Blueprints/BP_FirstPersonPlayerController` (`GameplayStatics.GetPlayerController` 0)))
      (set `self.PlayerInfoRef` (`/Game/FirstPerson/Blueprints/BP_FirstPersonPlayerController.PlayerInfo` _asbp_first_person_player_controller_2)))))

(event `SetPlayerInfo`
  (params (PlayerInfo :type "/Game/Blueprint/Widget/WBP_PlayerInfo Object Reference"))
  (set `self.PlayerInfoRef` PlayerInfo))

(event `/Game/Blueprint/Interface/BPI_Interactable.Interacting`
  (bind _returnvalue (`GameplayStatics.GetPlayerCharacter` 0))
  (bind _returnvalue_2 (`GameplayStatics.GetPlayerCharacter` 0))
  (bind _startscene (`self.StartScene`))
  (bind _returnvalue_3 (`self.K2_GetActorLocation` _returnvalue))
  (bind (_returnvalue_roll _returnvalue_pitch _returnvalue_yaw) (`KismetMathLibrary.BreakRotator` (`self.K2_GetActorRotation` _returnvalue_2)))
  (bind (_returnvalue_roll_2 _returnvalue_pitch_2 _returnvalue_yaw_2) (`KismetMathLibrary.BreakRotator` (`SceneComponent.K2_GetComponentRotation` _startscene)))
  (bind _returnvalue_4 (`self.K2_GetActorLocation` _returnvalue_2))
  (if (`self.Active`)
    (bind (_direction _delta) (`Timeline|Timeline`)
      (:`Update`
        (`SceneComponent.K2_SetRelativeRotation` (`self.Vintage_Office_Door_polySurface20`) (`KismetMathLibrary.MakeRotator` 0.0 0.0 _delta) false false)
        (`/Engine/EditorBlueprintResources/StandardMacros.DoOnce` false
          (:`Completed`
            (`|ExecutionSequence`
              (:`then_0`
                (bind _asbp_first_person_player_controller (cast `/Game/FirstPerson/Blueprints/BP_FirstPersonPlayerController` (`GameplayStatics.GetPlayerController` 0)))
                (`/Game/FirstPerson/Blueprints/BP_FirstPersonPlayerController.ShowResultScreen` _asbp_first_person_player_controller true 0.0)
                (bind _asbp_game_instance (cast `/Game/FirstPerson/Blueprints/BP_GameInstance` (`GameplayStatics.GetGameInstance`)))
                (`/Game/FirstPerson/Blueprints/BP_GameInstance.CheckAchievements` _asbp_game_instance true)
                (`/Engine/EditorBlueprintResources/StandardMacros.IsValid` (`self.PlayerInfoRef`)
                  (:`Is Valid`
                    (set `/Game/Blueprint/Widget/WBP_PlayerInfo.Completed` true (`self.PlayerInfoRef`))
                    (bind _asbp_game_instance_2 (cast `/Game/FirstPerson/Blueprints/BP_GameInstance` (`GameplayStatics.GetGameInstance`)))
                    (`/Game/FirstPerson/Blueprints/BP_GameInstance.SetBestTime` _asbp_game_instance_2 (`/Game/Blueprint/Widget/WBP_PlayerInfo.Second` (`self.PlayerInfoRef`))))))
              (:`then_1`
                (`/Engine/EditorBlueprintResources/StandardMacros.IsValid` (`self.PointLight`)
                  (:`Is Valid`
                    (bind (_direction_2 _lightintesity) (`Timeline|pointlightintensity`)
                      (:`Update`
                        (`LightComponent.SetIntensity` (`PointLight.PointLightComponent` (`self.PointLight`)) (* _lightintesity (`self.LightIntensity`))))))))
              (:`then_2`
                (bind (_direction_3 _playeroffset) (`Timeline|look at door`)
                  (:`Update`
                    (bind (_returnvalue_x _returnvalue_y) (`KismetMathLibrary.BreakVector` (`KismetMathLibrary.VLerp` _returnvalue_4 (`SceneComponent.K2_GetComponentLocation` _startscene) _playeroffset)))
                    (`self.K2_SetActorLocationAndRotation` _returnvalue_2 (`KismetMathLibrary.MakeVector` _returnvalue_x _returnvalue_y (.z _returnvalue_4)) (`KismetMathLibrary.MakeRotator` 0.0 0.0 (`KismetMathLibrary.Lerp` _returnvalue_yaw _returnvalue_yaw_2 _playeroffset)) false false))
                  (:`Finished`
                    (bind (_direction_4 _playeroffset_2) (`Timeline|intotheroom`)
                      (:`Update`
                        (bind (_returnvalue_x_2 _returnvalue_y_2) (`KismetMathLibrary.BreakVector` (`KismetMathLibrary.VLerp` _returnvalue_3 (`SceneComponent.K2_GetComponentLocation` (`self.EndScene`)) _playeroffset_2)))
                        (`self.K2_SetActorLocation` _returnvalue (`KismetMathLibrary.MakeVector` _returnvalue_x_2 _returnvalue_y_2 (.z _returnvalue_3)) false false)))))))))))
    (else
      (`GameplayStatics.PlaySoundAtLocation` "/Game/Sounds/Doors/Door_Locked_wav.Door_Locked_wav" (`self.K2_GetActorLocation`) (struct) 1.0 1.0 0.0 null null null null)
      (bind (_direction_5 _delta_2) (`Timeline|Timeline_0` :!via `PlayFromStart`)
        (:`Update`
          (`SceneComponent.K2_SetRelativeRotation` (`self.Vintage_Office_Door_polySurface20`) (`KismetMathLibrary.MakeRotator` 0.0 0.0 _delta_2) false false))))))

(fn `GetSoundLevel`
  (returns (SoundLevel :type "Float (double-precision)"))
  (return 0.0))

(fn `UserConstructionScript`)