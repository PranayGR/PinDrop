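; BP_InteractableSpawner is a spawner actor that places one randomly chosen actor class at its own location.
; BeginPlay picks the class from a list of candidates.
; SpawnEnemy spawns it only when no valid reference exists, adjusting for collision, and DestroyEnemy destroys it and clears the reference.
; GetSoundLevel returns zero, and the SpawnActor event and construction-time spawn logic are unused.
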(event `self.ReceiveBeginPlay`
  (set `self.Actor_Class` (`KismetArrayLibrary.Array_Random` (`self.Actor`))))

(event `/Game/Blueprint/Interface/BPI_Interactable.SpawnEnemy`
  (`self.ItemRef`
    (:`then`)
    (:`else`
      (bind _returnvalue (`|SpawnActorFromClass` (`self.Actor_Class`) (`KismetMathLibrary.MakeTransform` (`self.K2_GetActorLocation`)) "AdjustIfPossibleButAlwaysSpawn" "MultiplyWithRoot" null null))
      (set `self.ItemRef` _returnvalue))))

(event `SpawnActor`)

(event `/Game/Blueprint/Interface/BPI_Interactable.DestroyEnemy`
  (bind _itemref (`self.ItemRef`)
    (:`then`
      (`self.K2_DestroyActor` _itemref)
      (set `self.ItemRef` null))
    (:`else`)))

(fn `GetSoundLevel`
  (returns (SoundLevel :type "Float (double-precision)"))
  (return 0.0))

(fn `UserConstructionScript`)