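; BP_Chains is a chain actor that makes audible and AI-detectable noise when its Collided event is called.
; Collided plays a hit sound at the actor's location, scaled by the saved SFX level from BP_GameInstance, and reports a noise event there.
; A boolean gate with delays suppresses noise briefly after BeginPlay and adds a short cooldown between hits.
; Nothing in this Blueprint triggers Collided itself.
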(event `self.ReceiveBeginPlay`
  (set `self.CangenerateSoundAgain` false)
  (`KismetSystemLibrary.Delay` 5.0)
  (set `self.CangenerateSoundAgain` true))

(event `/Game/Blueprint/Interface/BPI_Interactable.Collided`
  (params (Velocity :type "Float (double-precision)") (Walk_State :type "/Game/FirstPerson/Blueprints/E_Movement Enum" :default "NewEnumerator0"))
  (bind _returnvalue (`self.K2_GetActorLocation`))
  (if (`self.CangenerateSoundAgain`)
    (set `self.CangenerateSoundAgain` false)
    (`GameplayStatics.PlaySoundAtLocation` "/Game/Sounds/On_Collide_with_Chains/on_hit_chain_1_wav.on_hit_chain_1_wav" _returnvalue (struct) (`/Game/FirstPerson/Blueprints/BP_SaveSlot.SFXLevel` (`/Game/FirstPerson/Blueprints/BP_GameInstance.SaveSlotRef` (cast `/Game/FirstPerson/Blueprints/BP_GameInstance` (`GameplayStatics.GetGameInstance`) :!pure true))) 1.0 0.0 null null null null)
    (`AISense_Hearing.ReportNoiseEvent` _returnvalue 1.0 self)
    (`KismetSystemLibrary.Delay` 0.5)
    (set `self.CangenerateSoundAgain` true)))

(fn `UserConstructionScript`
  (`parent.UserConstructionScript`))