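; BP_EnemySpawner spawns a single BP_Enemy at its own transform and carries the sound level between spawns.
; SpawnEnemy passes the current and maximum sound levels to the enemy and gives it a back-reference to the spawner.
; CanSpawnEnemyAgain stores a supplied level, re-arms spawning and starts a looping timer that steadily lowers the level toward zero.
; UpdateCurrentLevel and GetSoundLevel are stubs.
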(event `/Game/Blueprint/Interface/BPI_Interactable.SpawnEnemy`
  (if (not (`self.AlreadySpawn`))
    (bind _returnvalue (`|SpawnActorFromClass` "/Game/Blueprint/Enemy/BP_Enemy.BP_Enemy_C" (`KismetMathLibrary.MakeTransform` (`self.K2_GetActorLocation`) (`self.K2_GetActorRotation`)) "Undefined" "MultiplyWithRoot" self (`self.MaxSoundTolerance`) (`self.CurrentSoundLevel`) null))
    (set `self.EnemyRef` _returnvalue)
    (set `self.AlreadySpawn` true)
    (`/Engine/EditorBlueprintResources/StandardMacros.IsValid` (`self.EnemyRef`)
      (:`Is Valid`
        (set `/Game/Blueprint/Enemy/BP_Enemy.SpawnerRef` self (`self.EnemyRef`))))))

(event `CanSpawnEnemyAgain`
  (params (CurrentSoundLevel :type "Float (double-precision)"))
  (set `self.CurrentSoundLevel` CurrentSoundLevel)
  (set `self.AlreadySpawn` false)
  (set `self.EnemyRef` null)
  (`self.DecreaseSoundLevel`))

(event `DecreaseSoundLevel`
  (bind _returnvalue (`KismetSystemLibrary.K2_SetTimerDelegate` (delegate `DecreasingSoundlevel`) 0.5 true))
  (set `self.Dcreasehandle` _returnvalue))

(event `DecreasingSoundlevel`
  (set `self.CurrentSoundLevel` (`KismetMathLibrary.FClamp` (- (`self.CurrentSoundLevel`) (`self.DecresingRate`)) 0.0 (`self.MaxSoundTolerance`))))

(fn `GetSoundLevel`
  (returns (SoundLevel :type "Float (double-precision)"))
  (return 0.0))

(fn `UpdateCurrentLevel`
  (params (Value :type "Float (double-precision)")))

(fn `UserConstructionScript`)