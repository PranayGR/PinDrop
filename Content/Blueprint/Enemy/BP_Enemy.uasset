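; Zombie enemy that builds an alert level from heard noises, sight of the player and contact, shown on a widget bar.
; Gain scales around an intensity threshold that triggers disturbed animation and warning sound; timers drive sight buildup and decay.
; At maximum it sets Blackboard attack keys and alerts the game mode.
; Montages halt movement, attacks damage via timed hand sphere traces, stuns freeze it, and unalerted zombies can return to their spawner.
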(event `self.ReceiveBeginPlay`
  (`self.ChangeSpeed` false (`self.Stuned`))
  (bind _aswbp_alert_level (cast `/Game/Blueprint/Widget/WBP_AlertLevel` (`WidgetComponent.GetWidget` (`self.Widget`))))
  (set `self.WidgetRef` _aswbp_alert_level)
  (bind _asabp_zombie (cast `/Game/Zombie/ABP_Zombie` (`SkeletalMeshComponent.GetAnimInstance` (`self.Mesh`))))
  (set `self.AnimationRef` _asabp_zombie))

(event `self.AIPerception.OnTargetPerceptionUpdated`
  (params (Actor :type "Actor Object Reference") (Stimulus :type "AIStimulus Structure"))
  (bind _returnvalue (`AIPerceptionSystem.GetSenseClassForStimulus` Stimulus))
  (if (== _returnvalue "/Script/AIModule.AISense_Hearing")
    (`self.SoundUpdate` Actor Stimulus)
    (else
      (`self.UpdateVision` Actor Stimulus))))

(event `UpdateAlertLevel`
  (params (Level :type "Float (double-precision)"))
  (bind _returnvalue (`AIBlueprintHelperLibrary.GetBlackboard` (`AIBlueprintHelperLibrary.GetAIController` self)))
  (bind _returnvalue_2 (* Level (`KismetMathLibrary.SelectFloat` 1.0 (`self.IntensityBy`) (> (`self.CurrentSoundLevel`) (`self.IntensityThreshold`)))))
  (`self.ShowWidget` _returnvalue_2)
  (`self.UpdateCurrentLevel` (+ (`self.CurrentSoundLevel`) _returnvalue_2))
  (if (== (`self.CurrentSoundLevel`) (`self.MaxSoundTolerance`))
    (`KismetSystemLibrary.K2_ClearAndInvalidateTimerHandle` (`self.Dcreasehandle`))
    (`/Engine/EditorBlueprintResources/StandardMacros.DoOnce` false
      (:`Completed`
        (bind _asbp_first_person_character (cast `/Game/FirstPerson/Blueprints/BP_FirstPersonCharacter` (`GameplayStatics.GetPlayerCharacter` 0)))
        (add `/Game/FirstPerson/Blueprints/BP_FirstPersonCharacter.on_reached_safely` _asbp_first_person_character (delegate `StopEnemyMovement`))
        (set `self.Alerted` true)
        (`BlackboardComponent.SetValueAsObject` _returnvalue "Player" (`GameplayStatics.GetPlayerCharacter` 0))
        (`BlackboardComponent.SetValueAsBool` _returnvalue "Attack" true)
        (bind _asbp_first_person_game_mode (cast `/Game/FirstPerson/Blueprints/BP_FirstPersonGameMode` (`GameplayStatics.GetGameMode`)))
        (`/Game/FirstPerson/Blueprints/BP_FirstPersonGameMode.SetZombieAlerted` _asbp_first_person_game_mode true)
        ;[1 1 1] Time Require to Hide Bar
        (`KismetSystemLibrary.Delay` 5.0)
        (`Widget.SetVisibility` (`self.WidgetRef`) "Hidden")))
    (else
      ;[1 1 1] Time required Going Back to Normal
      (`KismetSystemLibrary.K2_SetTimerDelegate` (`|CreateDelegate` :!event `DecreaseSoundLevel`) 3.0))))

(event `SoundUpdate`
  (params (Actor :type "Actor Object Reference") (Stimuli :type "AIStimulus Structure"))
  (if (`.bSuccessfullySensed` (break `AIStimulus` Stimuli))
    (bind _soundlevel (message `/Game/Blueprint/Interface/BPI_Interactable.GetSoundLevel` Actor))
    (`self.UpdateAlertLevel` _soundlevel)))

(event `StopEnemyMovement`
  (set `CharacterMovementComponent.BrakingDecelerationWalking` 5000.0 (`self.CharacterMovement`)))

(event `UpdateVision`
  (params (Actor :type "Actor Object Reference") (Stimuli :type "AIStimulus Structure"))
  (if (`.bSuccessfullySensed` (break `AIStimulus` Stimuli))
    (cast `/Game/FirstPerson/Blueprints/BP_FirstPersonCharacter` Actor)
    (if (not (`KismetSystemLibrary.K2_IsValidTimerHandle` (`self.DetectedTimerHandle`)))
      (bind _returnvalue (`KismetSystemLibrary.K2_SetTimerDelegate` (delegate `Detected`) 0.1 true))
      (set `self.DetectedTimerHandle` _returnvalue))
    (else
      (cast `/Game/FirstPerson/Blueprints/BP_FirstPersonCharacter` Actor)
      (`KismetSystemLibrary.K2_ClearAndInvalidateTimerHandle` (`self.DetectedTimerHandle`)))))

(event `ShowWidget`
  (params (`Sound Level` :type "Float (double-precision)"))
  (if (> `Sound Level` (`self.ShowbarThreshold`))
    (`SceneComponent.SetVisibility` (`self.Widget`) true false)
    (`KismetSystemLibrary.K2_SetTimerDelegate` (delegate `HideBar`) 5.0)))

(event `Detected`
  ;[1 1 1] Detection Rate
  (`self.UpdateAlertLevel` 2.0))

(event `HideBar`
  (`SceneComponent.SetVisibility` (`self.Widget`) false false))

(event `DecreaseSoundLevel`
  ;[1 1 1] Decreasing - Going Back to Noraml
  (bind _returnvalue (`KismetSystemLibrary.K2_SetTimerDelegate` (delegate `DecreasingSoundlevel`) 0.5 true))
  (set `self.Dcreasehandle` _returnvalue))

(event `DecreasingSoundlevel`
  ;[1 1 1] Decreasing - Going Back to Noraml
  (`self.UpdateCurrentLevel` (- (`self.CurrentSoundLevel`) (`self.DecresingRate`))))

(event `/Game/Blueprint/Interface/BPI_Interactable.VisualEnable`
  (params (Hidden :type Boolean))
  (`self.SetActorHiddenInGame` Hidden))

(event `Attack`
  (if (not (`self.Attacking`))
    (set `self.Attacking` true)
    (set `/Game/Zombie/ABP_Zombie.Attacking` true (`self.AnimationRef`))
    ;[1 1 1] Attack Rate -- Play Rate
    (`|PlayMontage` (`self.Mesh`) (`KismetArrayLibrary.Array_Random` (`self.AttackMontage`)) 1.2 0.0 "Start"
      (:`then`
        (`self.ChangeSpeed` true (`self.Stuned`)))
      (:`OnCompleted`
        (set `self.Attacking` false :!label _label)
        (set `/Game/Zombie/ABP_Zombie.Attacking` false (`self.AnimationRef`))
        (`self.ChangeSpeed` false (`self.Stuned`)))
      (:`OnBlendOut`
        (goto _label))
      (:`OnInterrupted`
        (goto _label)))))

(event `Roar`
  (bind _stuned (`self.Stuned`))
  ;[1 1 1] Roar Animation - Change Play Rate
  (`|PlayMontage` (`self.Mesh`) "/Game/Zombie/Animation/Anim/Run_Chase/Zombie_Scream_Montage.Zombie_Scream_Montage" 1.2
    (:`then`
      (`self.ChangeSpeed` true _stuned))
    (:`OnCompleted`
      (`self.ChangeSpeed` false _stuned :!label _label_2))
    (:`OnBlendOut`
      (goto _label_2))
    (:`OnInterrupted`
      (goto _label_2))))

(event `EnableLineTrace`
  (params (Enable :type Boolean) (RightHand :type Boolean) (Lefthand :type Boolean))
  (if Enable
    (bind _returnvalue (`KismetSystemLibrary.K2_SetTimerDelegate` (delegate `LineTraceLoop`) 0.02 true))
    (set `self.LineTraceHandle` _returnvalue)
    (else
      (`KismetSystemLibrary.K2_ClearAndInvalidateTimerHandle` (`self.LineTraceHandle`)))))

(event `LineTraceLoop`
  (`|ExecutionSequence`
    (:`then_0`
      (if (stale `EnableLineTrace` RightHand)
        (`self.CheckLineTraceHit` (`self.RightHand`))))
    (:`then_1`
      (if (stale `EnableLineTrace` Lefthand)
        (`self.CheckLineTraceHit` (`self.LeftHand`))))))

(event `/Game/Blueprint/Interface/BPI_Interactable.DestroyEnemy`
  (bind _spawnerref (`self.SpawnerRef`))
  (if (not (`self.Alerted`))
    (`/Engine/EditorBlueprintResources/StandardMacros.IsValid` _spawnerref
      (:`Is Valid`
        (`/Game/Blueprint/Enemy/BP_EnemySpawner.CanSpawnEnemyAgain` _spawnerref (`self.CurrentSoundLevel`))
        (`self.K2_DestroyActor`)))))

(event `/Game/Blueprint/Interface/BPI_Interactable.Collided`
  (params (Velocity :type "Float (double-precision)") (Walk_State :type "/Game/FirstPerson/Blueprints/E_Movement Enum" :default "NewEnumerator0"))
  ;[1 1 1] Check this - Contact with zombie
  (`self.UpdateAlertLevel` 40.0))

(event `/Game/Blueprint/Interface/BPI_Interactable.Stun`
  (params (Stun :type Boolean) (NoBattery :type Boolean))
  (bind _output_get (set `self.Stuned` Stun))
  (if _output_get
    (if NoBattery
      (`self.ChangeSpeed` false)
      (else
        (`self.ChangeSpeed` true true)))
    (elif (`self.Alerted`)
      (if NoBattery
        (`self.ChangeSpeed` false :!label _label_3)
        (else
          (`KismetSystemLibrary.K2_SetTimerDelegate` (delegate `Reset_Stun`) (`self.StunTimer`)))))))

(event `Reset_Stun`
  (goto _label_3))

(fn `ChangeSpeed`
  (params (StopMovement :type Boolean) (Stunned :type Boolean))
  (if StopMovement
    (`NavMovementComponent.StopActiveMovement` (`self.CharacterMovement`) :!label _label)
    (set `CharacterMovementComponent.MaxWalkSpeed` 0.0 (`self.CharacterMovement`))
    (if (`self.Alerted`)
      _)
    (elif Stunned
      (goto _label)
      (else
        (set `CharacterMovementComponent.MaxWalkSpeed` (`self.Max Walk Speed`) (`self.CharacterMovement`))
        (if (`self.Alerted`)
          _)))))

(fn `CheckLineTraceHit`
  (params (Hand :type "SceneComponent Object Reference"))
  (bind _returnvalue (`SceneComponent.K2_GetComponentLocation` Hand))
  (if (`self.Attacking`)
    (bind (_outhit _returnvalue_2) (`KismetSystemLibrary.SphereTraceSingleByProfile` _returnvalue _returnvalue 40.0 "None" false (`|MakeArray` self :!type "Actor Object Reference")))
    (if _returnvalue_2
      (bind (_bblockinghit _binitialoverlap _time _distance _location _impactpoint _normal _impactnormal _physmat _hitactor) (`GameplayStatics.BreakHitResult` _outhit))
      (cast `/Game/FirstPerson/Blueprints/BP_FirstPersonCharacter` _hitactor)
      (`KismetSystemLibrary.K2_ClearAndInvalidateTimerHandle` (`self.LineTraceHandle`))
      (`GameplayStatics.ApplyDamage` _hitactor 10.0))))

(fn `GetSoundLevel`
  (returns (SoundLevel :type "Float (double-precision)"))
  (return 0.0))

(fn `UpdateCurrentLevel`
  (params (Value :type "Float (double-precision)"))
  (set `self.CurrentSoundLevel` (`KismetMathLibrary.FClamp` Value 0.0 (`self.MaxSoundTolerance`)))
  (`/Game/Blueprint/Widget/WBP_AlertLevel.UpdateAlertBar` (`self.WidgetRef`) (/ (`self.CurrentSoundLevel`) (`self.MaxSoundTolerance`)))
  (if (>= (`self.CurrentSoundLevel`) (`self.IntensityThreshold`))
    (`/Engine/EditorBlueprintResources/StandardMacros.DoOnce` false :!label _label
      (:`Completed`
        (`|ExecutionSequence`
          (:`then_0`
            (set `/Game/Zombie/ABP_Zombie.Disturb` true (`self.AnimationRef`))
            (bind _asbp_first_person_game_mode (cast `/Game/FirstPerson/Blueprints/BP_FirstPersonGameMode` (`GameplayStatics.GetGameMode`)))
            (`/Game/FirstPerson/Blueprints/BP_FirstPersonGameMode.PlayWarningSound` _asbp_first_person_game_mode))
          (:`then_1`
            (goto _label_2 :!via `Reset`)))))
    (else
      (`/Engine/EditorBlueprintResources/StandardMacros.DoOnce` false :!label _label_2
        (:`Completed`
          (`|ExecutionSequence`
            (:`then_0`
              (set `/Game/Zombie/ABP_Zombie.Disturb` false (`self.AnimationRef`)))
            (:`then_1`
              (goto _label :!via `Reset`))))))))

(fn `UserConstructionScript`)