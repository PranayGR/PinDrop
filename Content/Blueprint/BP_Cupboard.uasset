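; BP_Cupboard is an interactable cupboard that may hold a battery pickup for the first-person player.
; On BeginPlay it randomly decides, with roughly 80% odds, whether a battery is present and shows or hides the Cube mesh accordingly.
; Interacting, gated by HasBattery and a one-shot Used flag, hides the battery, plays a sound, replenishes player energy, and flags the pickup on the character and game mode.
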(event `self.ReceiveBeginPlay`
  (`parent.ReceiveBeginPlay`)
  (if (> (`KismetMathLibrary.RandomFloatInRange` 0.0 1.0) 0.2)
    (`self.set_active_battery` true)
    (else
      (`self.set_active_battery` false))))

(event `/Game/Blueprint/Interface/BPI_Interactable.Interacting`
  (if (`self.HasBattery`)
    (if (`self.used`)
      (set `self.used` false)
      (`SceneComponent.SetHiddenInGame` (`self.Cube`) true false)
      (bind _asbp_first_person_character (cast `/Game/FirstPerson/Blueprints/BP_FirstPersonCharacter` (`GameplayStatics.GetPlayerCharacter` 0)))
      (set `/Game/FirstPerson/Blueprints/BP_FirstPersonCharacter.BatteryPicked` true _asbp_first_person_character)
      (`GameplayStatics.PlaySound2D` "/Game/Sounds/Torch/battery-pickup_wav.battery-pickup_wav" 1.0 1.0 0.0 null null)
      (`/Game/FirstPerson/Blueprints/BP_FirstPersonCharacter.ReplinishEnergy` _asbp_first_person_character)
      (bind _asbp_first_person_game_mode (cast `/Game/FirstPerson/Blueprints/BP_FirstPersonGameMode` (`GameplayStatics.GetGameMode`)))
      (`/Game/FirstPerson/Blueprints/BP_FirstPersonGameMode.SetBatteryPicked` _asbp_first_person_game_mode true))))

(fn `set_active_battery`
  (params (Active :type Boolean))
  (if Active
    (set `self.HasBattery` true)
    (`SceneComponent.SetHiddenInGame` (`self.Cube`) false false)
    (else
      (set `self.HasBattery` false)
      (`SceneComponent.SetHiddenInGame` (`self.Cube`) true false))))

(fn `UserConstructionScript`
  (`parent.UserConstructionScript`))