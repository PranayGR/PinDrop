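; BP_Chains2 is a chain prop that makes noise when struck.
; Its Collided event takes a velocity and, at or above a threshold, plays a chain hit sound at the actor's location, scaled by the saved SFX level from the game instance.
; It also reports a noise event at that spot with itself as instigator, so AI hearing can pick it up.
; GetSoundLevel returns zero.
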(event `/Game/Blueprint/Interface/BPI_Interactable.Collided`
  (params (Velocity :type "Float (double-precision)") (Walk_State :type "/Game/FirstPerson/Blueprints/E_Movement Enum" :default "NewEnumerator0"))
  (bind _returnvalue (`self.K2_GetActorLocation`))
  (if (>= Velocity 50.0)
    (`GameplayStatics.PlaySoundAtLocation` "/Game/Sounds/On_Collide_with_Chains/on_hit_chain_2_wav.on_hit_chain_2_wav" _returnvalue (struct) (`/Game/FirstPerson/Blueprints/BP_SaveSlot.SFXLevel` (`/Game/FirstPerson/Blueprints/BP_GameInstance.SaveSlotRef` (cast `/Game/FirstPerson/Blueprints/BP_GameInstance` (`GameplayStatics.GetGameInstance`) :!pure true))) 1.0 0.0 null null null null)
    (`AISense_Hearing.ReportNoiseEvent` _returnvalue 1.0 self)))

(fn `GetSoundLevel`
  (returns (SoundLevel :type "Float (double-precision)"))
  (return 0.0))

(fn `UserConstructionScript`)