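; BP_Door is an interactable door that is either the active "true" door or a locked decoy, defaulting to locked on construction.
; Interacting updates the player's door count, then either flip-flops an opening timeline and triggers achievements, or plays a locked sound and shake and records the find in the game instance.
; SpawnHallway loads a hallway level instance at the door's transform, and its box overlap notifies the player character it reached safety.
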(event `self.ReceiveBeginPlay`
  (bind _asbp_first_person_player_controller (cast `/Game/FirstPerson/Blueprints/BP_FirstPersonPlayerController` (`GameplayStatics.GetPlayerController` 0)))
  (add `/Game/FirstPerson/Blueprints/BP_FirstPersonPlayerController.PlayerInfoAdded` _asbp_first_person_player_controller (delegate `SetPlayerInfo`))
  (bind _asbp_game_instance (cast `/Game/FirstPerson/Blueprints/BP_GameInstance` (`GameplayStatics.GetGameInstance`)))
  (set `self.GameInstanceRef` _asbp_game_instance))

(event `SpawnHallway`
  (bind (_boutsuccess _returnvalue) (`LevelStreamingDynamic.LoadLevelInstanceBySoftObjectPtr` "/Game/Map/Hallway.Hallway" (`self.K2_GetActorLocation`) (`self.K2_GetActorRotation`) "" null))
  (set `self.LevelInstRef` _returnvalue))

(event `SetPlayerInfo`
  (params (PlayerInfo :type "/Game/Blueprint/Widget/WBP_PlayerInfo Object Reference"))
  (set `self.PlayerInfoRef` PlayerInfo))

(event `/Game/Blueprint/Interface/BPI_Interactable.Interacting`
  (`self.GameInstanceRef`
    (:`then`
      (`/Engine/EditorBlueprintResources/StandardMacros.IsValid` (`self.PlayerInfoRef`)
        (:`Is Valid`
          (`/Game/Blueprint/Widget/WBP_PlayerInfo.DoorCoundUpdated` (`self.PlayerInfoRef`)))
        (:`Is Not Valid`
          _))
      (if (`self.Active`)
        (`|ExecutionSequence`
          (:`then_0`
            ;[1 1 1] Door Opening Timeline
            (`/Engine/EditorBlueprintResources/StandardMacros.FlipFlop`
              (:`A`
                (bind (_direction _delta) (`Timeline|DoorOpening` :!label _label)
                  (:`Update`
                    (`SceneComponent.K2_SetRelativeRotation` (`self.Door`) (`KismetMathLibrary.MakeRotator` 0.0 0.0 (- 180.0 _delta)) false false))))
              (:`B`
                (goto _label :!via `Reverse`))))
          (:`then_1`
            ;[1 1 1] Achievements
            (`/Game/FirstPerson/Blueprints/BP_GameInstance.FoundTrueDoor` (`self.GameInstanceRef`))
            (`/Game/FirstPerson/Blueprints/BP_GameInstance.CheckAchievements` (`self.GameInstanceRef`) true)))
        (else
          (`GameplayStatics.PlaySoundAtLocation` "/Game/Sounds/Doors/Door_Locked_wav.Door_Locked_wav" (`self.K2_GetActorLocation`) (struct) 1.0 1.0 0.0 null null null null)
          (`/Game/FirstPerson/Blueprints/BP_GameInstance.AddFoundLockedDoor` (`self.GameInstanceRef`) self)
          (bind (_direction_2 _delta_2) (`Timeline|DoorShake` :!via `PlayFromStart`)
            (:`Update`
              (`SceneComponent.K2_SetRelativeRotation` (`self.Door`) (`KismetMathLibrary.MakeRotator` 0.0 0.0 (- 180.0 _delta_2)) false false))))))
    (:`else`)))

(event `self.Box.OnComponentBeginOverlap`
  (params (OverlappedComponent :type "PrimitiveComponent Object Reference") (OtherActor :type "Actor Object Reference") (OtherComp :type "PrimitiveComponent Object Reference") (OtherBodyIndex :type Integer) (bFromSweep :type Boolean) (SweepResult :type "HitResult Structure (by ref)"))
  (bind _asbp_first_person_character (cast `/Game/FirstPerson/Blueprints/BP_FirstPersonCharacter` OtherActor))
  (`/Game/FirstPerson/Blueprints/BP_FirstPersonCharacter.on_reached_safely` _asbp_first_person_character))

(fn `GetSoundLevel`
  (returns (SoundLevel :type "Float (double-precision)"))
  (return 0.0))

(fn `UpdateMaterial`
  (params (Active :type Boolean))
  (set `self.Active` Active))

(fn `UserConstructionScript`
  (`self.UpdateMaterial` false))