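; BP_ChainSpawner is an actor that spawns and removes a single BP_Chains2 chain actor on demand.
; Its SpawnChain event takes a boolean: true spawns a chain slightly below the spawner with its rotation, unless one already exists, and false destroys it and clears the stored reference.
; GetSoundLevel is a stub that returns zero.
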(event `/Game/Blueprint/Interface/BPI_Interactable.SpawnChain`
  (params (Spawn :type Boolean))
  (bind (_returnvalue_x _returnvalue_y _returnvalue_z) (`KismetMathLibrary.BreakVector` (`self.K2_GetActorLocation`)))
  (if Spawn
    (`/Engine/EditorBlueprintResources/StandardMacros.IsValid` (`self.ChainRef`)
      (:`Is Not Valid`
        (bind _returnvalue (`|SpawnActorFromClass` "/Game/Blueprint/BP_Chains2.BP_Chains2_C" (`KismetMathLibrary.MakeTransform` (`KismetMathLibrary.MakeVector` _returnvalue_x _returnvalue_y (- _returnvalue_z 50.0)) (`self.K2_GetActorRotation`)) "Undefined" "MultiplyWithRoot" null null))
        (set `self.ChainRef` _returnvalue)))
    (else
      (`/Engine/EditorBlueprintResources/StandardMacros.IsValid` (`self.ChainRef`)
        (:`Is Valid`
          (`self.K2_DestroyActor` (`self.ChainRef`))
          (set `self.ChainRef` null))))))

(fn `GetSoundLevel`
  (returns (SoundLevel :type "Float (double-precision)"))
  (return 0.0))

(fn `UserConstructionScript`)