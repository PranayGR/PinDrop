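; Room actor that builds a procedurally generated room with one true exit door and a battery supply in its cupboards.
; On BeginPlay it runs PCG_Item on the level's PCGVolume with a random seed, then polls each tick until four BP_Door actors exist.
; UpdateDoor marks a random door as true and spawns its hallway.
; After a short delay, BatteryCountCheck activates batteries in random cupboards if too few have one.
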(event EventBeginPlay
  (bind _returnvalue (Actor|GetActorOfClass "/Script/PCG.PCGVolume"))
  (Class|PCGComponent|SetGraph (Variables|/Script/PCG.PCGVolume|GetPCGComponent _returnvalue) "/Game/PCG/PCG_Item.PCG_Item")
  (Variables|/Script/PCG.PCGComponent|SetSeed (Variables|/Script/PCG.PCGVolume|GetPCGComponent _returnvalue) (Math|Random|RandomInteger 10000))
  (PCG|Generate (Variables|/Script/PCG.PCGVolume|GetPCGComponent _returnvalue) true)
  (Class|AssetRegistry|WaitforCompletion(Message) (Variables|/Script/PCG.PCGVolume|GetPCGComponent _returnvalue))
  (bind _outactors (Actor|GetAllActorsOfClass "/Game/Blueprint/BP_Door.BP_Door_C" :!label _label))
  (if (== (Utilities|Array|Length _outactors) 4)
    (CallFunction|UpdateDoor)
    (Utilities|FlowControl|Delay 0.5)
    (CallFunction|BatteryCountCheck)
    (else
      (Utilities|FlowControl|DelayUntilNextTick)
      (goto _label))))

(fn ConstructionScript
  (if (not (Variables|Default|GetRegenerate))
    (Variables|Default|SetRoomSize (Variables|Default|GetRoomSize))
    (Variables|Default|SetRandomSeed (Math|Random|RandomInteger 10000))
    (Variables|Default|SetRegenerate true)))

(fn UpdateDoor
  (bind _outactors (Actor|GetAllActorsOfClass "/Game/Blueprint/BP_Door.BP_Door_C"))
  (for _array_element _outactors
    (Default|UpdateMaterial _array_element false))
  (Variables|Default|SetTrueDoor (.OutItem (Utilities|Array|Random _outactors)))
  (Default|UpdateMaterial (Variables|Default|GetTrueDoor) true)
  (Default|SpawnHallway (Variables|Default|GetTrueDoor)))

(fn BatteryCountCheck
  (bind _outactors (Actor|GetAllActorsOfClass "/Game/Blueprint/BP_Cupboard.BP_Cupboard_C"))
  (LocalVariables|SetItemArray _outactors)
  (for _array_element (LocalVariables|GetItemArray)
    (if (Variables|/Game/Blueprint/BP_Cupboard.BP_Cupboard_C|GetHasBattery _array_element)
      (Math|Integer|IncrementInt (LocalVariables|GetLocalBatteryCount))))
  (if (not (>= (LocalVariables|GetLocalBatteryCount) (Variables|Default|GetMinBatteryCount)))
    (if (> (Utilities|Array|Length (LocalVariables|GetItemArray)) (Variables|Default|GetMinBatteryCount))
      (for _index (range 1 (Variables|Default|GetMinBatteryCount))
        (LocalVariables|SetTemp (.OutItem (Utilities|Array|Random (LocalVariables|GetItemArray))))
        (Utilities|Array|RemoveItem (LocalVariables|GetItemArray) (.OutItem (Utilities|Array|Random (LocalVariables|GetItemArray))))
        (Default|SetActiveBattery (.OutItem (Utilities|Array|Random (LocalVariables|GetItemArray))) true))
      (else
        (for _array_element_2 (LocalVariables|GetItemArray)
          (Default|SetActiveBattery _array_element_2 true))))))